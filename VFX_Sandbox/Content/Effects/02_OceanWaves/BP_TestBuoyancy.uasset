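; Test actor that mimics buoyancy by following the Gerstner wave surface of an ocean actor, without physics.
; Each tick it queries wave height, offset and normal at its location using fixed wave parameters.
; It interpolates X and Y toward the offset, Z toward starting height plus wave height, and rotation toward a normal-aligned basis built with cross products.
; Debug lines for normal, tangent and binormal are present but unconnected.
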(event EventBeginPlay
  (Variables|Default|SetinitialZ (.z (Transformation|GetActorLocation))))

(event Collision|EventActorBeginOverlap
  (params (OtherActor :type Actor%20Object%20Reference)))

(event EventTick
  (params (DeltaSeconds :type Float%20%28single-precision%29))
  (bind (_height _normal _tangent _binormal _offset) (Default|TryGetGerstnerWaveHeight (Variables|Default|GetOceanActor) (Transformation|GetActorLocation) 3e+01 "(X=1.000000,Y=2.000000)" 0.25 5))
  (Transformation|SetActorLocationAndRotation (Math|Interpolation|VInterpTo (Transformation|GetActorLocation) (Math|Vector|MakeVector (.X (Math|Vector|BreakVector _offset)) (.Y (Math|Vector|BreakVector _offset)) (+ (Variables|Default|GetinitialZ) _height)) DeltaSeconds 1e+01) (Math|Interpolation|RInterpTo (Transformation|GetWorldRotation (Variables|Default|GetDefaultSceneRoot)) (Math|Rotator|MakeRotationfromAxes (Math|Vector|CrossProduct (Math|Vector|CrossProduct (Math|Vector|MakeVector -1.0 0.0 0.0001) _normal) _normal) (Math|Vector|CrossProduct (Math|Vector|MakeVector -1.0 0.0 0.0001) _normal) _normal) DeltaSeconds 1e+01)))

(fn ConstructionScript)