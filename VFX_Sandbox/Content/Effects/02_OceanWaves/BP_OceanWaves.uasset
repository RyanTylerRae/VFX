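; BP_OceanWaves is an ocean wave Blueprint that evaluates a Gerstner wave at a world position.
; GetGerstnerWaveAt derives height, horizontal offset, tangent and binormal from wavelength, direction, steepness and game time, using gravity-based wave speed.
; TryGetGerstnerWaveHeight repeatedly subtracts the previous horizontal offset before re-evaluating, converging on the surface height at that position.
; The returned normal is the tangent with X and Y swapped; the cross-product normal is unused.
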(event EventBeginPlay)

(event Collision|EventActorBeginOverlap
  (params (OtherActor :type Actor%20Object%20Reference)))

(event EventTick
  (params (DeltaSeconds :type Float%20%28single-precision%29)))

(fn ConstructionScript)

(fn GetGerstnerWaveat
  (params (WorldPos :type Vector%202D%20Structure) (Wavelength :type Float%20%28double-precision%29) (Direction :type Vector%202D%20Structure) (Steepness :type Float%20%28double-precision%29))
  (bind (_x _y) (Math|Vector2D|BreakVector2D Direction))
  (Utilities|FlowControl|Sequence
    (:then_0
      (LocalVariables|SetinvWavelength (/ (Math|Float|MakeLiteralFloat 1.0) Wavelength)))
    (:then_1
      (LocalVariables|SetkVal (* (* (Math|Float|MakeLiteralFloat 2.0) 3.141596) (LocalVariables|GetinvWavelength))))
    (:then_2
      (LocalVariables|SetcVal (Math|Float|Sqrt (/ (Math|Float|MakeLiteralFloat 9.8) (LocalVariables|GetkVal)))))
    (:then_3
      (LocalVariables|SetfVal (* (LocalVariables|GetkVal) (- (Math|Vector2D|DotProduct(2D) (Class|KismetMathLibrary|NormalSafe2D Direction 0.0001) WorldPos) (* (Utilities|Time|GetGameTimeinSeconds) (LocalVariables|GetcVal))))))
    (:then_4
      (LocalVariables|SetaVal (/ Steepness (LocalVariables|GetkVal))))
    (:then_5
      (Utilities|FlowControl|Sequence
        (:then_0
          (LocalVariables|Setheight (* (LocalVariables|GetaVal) (Math|Trig|Sin(Radians) (LocalVariables|GetfVal)))))
        (:then_1
          (bind _output_get (LocalVariables|Setdx _x))
          (LocalVariables|Setdx2 (* _output_get _output_get)))
        (:then_2
          (bind _output_get_2 (LocalVariables|Setdy _y))
          (LocalVariables|Setdy2 (* _output_get_2 _output_get_2)))
        (:then_3
          (LocalVariables|Settangent (Math|Vector|MakeVector (- (Math|Float|MakeLiteralFloat 1.0) (* (LocalVariables|Getdx2) Steepness (Math|Trig|Sin(Radians) (LocalVariables|GetfVal)))) (* (Math|Float|MakeLiteralFloat -1.0) (LocalVariables|Getdx) (LocalVariables|Getdy) Steepness (Math|Trig|Sin(Radians) (LocalVariables|GetfVal))) (* (LocalVariables|Getdx) Steepness (Math|Trig|Cos(Radians) (LocalVariables|GetfVal))))))
        (:then_4
          (LocalVariables|Setbinormal (Math|Vector|MakeVector (* (Math|Float|MakeLiteralFloat -1.0) (LocalVariables|Getdx) (LocalVariables|Getdy) Steepness (Math|Trig|Sin(Radians) (LocalVariables|GetfVal))) (- (Math|Float|MakeLiteralFloat 1.0) (* (LocalVariables|Getdy2) Steepness (Math|Trig|Sin(Radians) (LocalVariables|GetfVal)))) (* (LocalVariables|Getdy) Steepness (Math|Trig|Cos(Radians) (LocalVariables|GetfVal))))))
        (:then_5
          (return (LocalVariables|Getheight) (Math|Vector|Normalize (Math|Vector|MakeVector (.Y (Math|Vector|BreakVector (Math|Vector|Normalize (LocalVariables|Gettangent)))) (Math|Float|MakeLiteralFloat (.X (Math|Vector|BreakVector (Math|Vector|Normalize (LocalVariables|Gettangent))))) (.Z (Math|Vector|BreakVector (Math|Vector|Normalize (LocalVariables|Gettangent)))))) (Math|Vector2D|MakeVector2D (* (.x Direction) (LocalVariables|GetaVal) (Math|Trig|Cos(Radians) (LocalVariables|GetfVal))) (* (.y Direction) (Math|Trig|Cos(Radians) (LocalVariables|GetfVal)) (LocalVariables|GetaVal))) (Math|Vector|Normalize (LocalVariables|Gettangent)) (Math|Vector|Normalize (LocalVariables|Getbinormal))))))))

(fn TryGetGerstnerWaveHeight
  (params (WorldPos :type Vector) (Wavelength :type Float%20%28double-precision%29) (Direction :type Vector%202D%20Structure) (Steepness :type Float%20%28double-precision%29) (Iterations :type Integer))
  (bind (_x _y) (Math|Vector|BreakVector WorldPos))
  (for _index (range 0 (- Iterations 1))
    (bind (_worldheight _normal _worldoffset _outtangent _outbinormal) (CallFunction|GetGerstnerWaveat (- (Math|Vector2D|MakeVector2D _x _y) (LocalVariables|GetOut_Offset)) Wavelength Direction Steepness))
    (LocalVariables|SetOut_Height _worldheight)
    (LocalVariables|SetOut_Normal _normal)
    (LocalVariables|SetOut_Offset _worldoffset)
    (LocalVariables|SetOut_Tangent _outtangent)
    (LocalVariables|SetOut_Binormal _outbinormal))
  (return (LocalVariables|GetOut_Height) (LocalVariables|GetOut_Normal) (LocalVariables|GetOut_Tangent) (LocalVariables|GetOut_Binormal) (Math|Vector|MakeVector (.x (LocalVariables|GetOut_Offset)) (.y (LocalVariables|GetOut_Offset)) 0.0)))