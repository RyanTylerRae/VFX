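; BP_HoverAndRotate is an actor whose static mesh bobs up and down while spinning around its vertical axis.
; Each tick it rebuilds the mesh's relative transform from the time since creation.
; A sine of that time, tuned by Speed and Displacement, sets the height, and RotationSpeed drives the yaw angle.
; The transform is absolute rather than accumulated, so it overrides any offset, rotation or scale set on the mesh.
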(event EventBeginPlay)

(event Collision|EventActorBeginOverlap
  (params (OtherActor :type Actor%20Object%20Reference)))

(event EventTick
  (params (DeltaSeconds :type Float%20%28single-precision%29))
  (bind _returnvalue (Actor|GetGameTimeSinceCreation))
  (Transformation|SetRelativeTransform (Variables|Default|GetStaticMesh) (Math|Transform|MakeTransform (Math|Vector|MakeVector 0.0 0.0 (* (Math|Trig|Sin(Radians) (* _returnvalue (Variables|Default|GetSpeed))) (Variables|Default|GetDisplacement))) (Math|Vector|RotatorfromAxisandAngle "0.000000,0.000000,1.000000" (* _returnvalue (Variables|Default|GetRotationSpeed)))) false false))

(fn ConstructionScript)